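; BP_Floor is a floor tile actor that signals the game mode when to spawn and destroy tiles.
; It caches the game mode on BeginPlay and uses two trigger volumes.
; Any valid actor entering Spawn_collision sends SpawnTilesMessage to the game mode.
; Any overlap with Destroy_collision sends DestroyTilesMessage, then the tile destroys itself.
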(event OnComponentBeginOverlap(Destroy_collision)
  (params (OverlappedComponent :type Primitive%20Component%20Object%20Reference) (OtherActor :type Actor%20Object%20Reference) (OtherComp :type Primitive%20Component%20Object%20Reference) (OtherBodyIndex :type Integer) (bFromSweep :type Boolean) (SweepResult :type Hit%20Result%20Structure%20%28by%20ref%29))
  (Class|BPISpawning|DestroyTiles(Message) (Variables|Default|GetGamemode_Ref))
  (Actor|DestroyActor))

(event OnComponentBeginOverlap(Spawn_collision)
  (params (OverlappedComponent :type Primitive%20Component%20Object%20Reference) (OtherActor :type Actor%20Object%20Reference) (OtherComp :type Primitive%20Component%20Object%20Reference) (OtherBodyIndex :type Integer) (bFromSweep :type Boolean) (SweepResult :type Hit%20Result%20Structure%20%28by%20ref%29))
  (Utilities|IsValid OtherActor
    (:Is%20Valid
      (Variables|Default|SetChar%20Ref (Variables|Default|GetChar%20Ref))
      (Class|BPISpawning|SpawnTiles(Message) (Variables|Default|GetGamemode_Ref)))))

(event EventBeginPlay
  (Variables|Default|SetGamemode_Ref (Game|GetGameMode)))

(fn ConstructionScript)