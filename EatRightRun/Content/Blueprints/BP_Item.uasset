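; BP_Item is a data-table-driven pickup, commented as a healthy or unhealthy item.
; The construction script sets mesh and scale from RowName, then BeginPlay replaces the mesh and material with a random row's, leaving scale unchanged.
; On box overlap it sends ItemData.ItemType to the other actor via ApplyItemTypeMessage and destroys itself.
; BeginPlay assigns None to ItemData rather than the chosen row, and starts a looping timer with no bound event.
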(event OnComponentBeginOverlap(Box)
  (params (OverlappedComponent :type Primitive%20Component%20Object%20Reference) (OtherActor :type Actor%20Object%20Reference) (OtherComp :type Primitive%20Component%20Object%20Reference) (OtherBodyIndex :type Integer) (bFromSweep :type Boolean) (SweepResult :type Hit%20Result%20Structure%20%28by%20ref%29))
  ;[0.15 0.15 0.15 0.5] Healthy/ Unhealthy Item.
  (Class|BPIItemInteraction|ApplyItemType(Message) OtherActor (.ItemType (Utilities|Struct|BreakItemData (Variables|Default|GetItemData))))
  (Actor|DestroyActor))

(event EventBeginPlay
  (bind _item (Variables|Default|GetItem))
  (Utilities|Time|SetTimerbyEvent 0 0.03 true)
  (bind _outrownames (DataTable|GetDataTableRowNames "/Game/ItemDataTable.ItemDataTable"))
  (bind _returnvalue (Utilities|GetDataTableRow "/Game/ItemDataTable.ItemDataTable" (.OutItem (Utilities|Array|Random _outrownames)))
    (:then
      (Variables|Default|SetItemData "")
      (Development|PrintString "Hello")
      (Components|StaticMesh|SetStaticMesh _item (.mesh _returnvalue))
      (Rendering|Material|SetMaterial _item 0 (.material _returnvalue)))))

(fn ConstructionScript
  (bind _item (Variables|Default|GetItem))
  (bind _returnvalue (Utilities|GetDataTableRow "/Game/ItemDataTable.ItemDataTable" (Variables|Default|GetRowName))
    (:then
      (Components|StaticMesh|SetStaticMesh _item (.Mesh (Utilities|Struct|BreakItemData _returnvalue)))
      (Transformation|SetRelativeScale3D _item (.MeshScale (Utilities|Struct|BreakItemData _returnvalue))))))